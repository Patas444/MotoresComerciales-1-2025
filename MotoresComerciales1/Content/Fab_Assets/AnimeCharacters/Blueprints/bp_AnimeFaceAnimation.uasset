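; Anime character face animation Blueprint that holds expression, eye look, eye emote, talking and look-at state.
; A single setter updates that state, while the look query returns the target actor's interface-provided look point, falling back to the actor's location.
; Eye emotes toggle an override morph target on the head mesh and swap textures from a map on a lazily created dynamic material in a named slot.
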(fn `CreateEyeEmoteDynamicMaterial`
  (params (HeadComp :type "SkeletalMeshComponent Object Reference"))
  (bind _returnvalue (`KismetArrayLibrary.Array_Find` (`MeshComponent.GetMaterialSlotNames` HeadComp) (`self.EyeEmoteSlotName`)))
  ;[1 1 1] Create EyeEmote Dynamic Material
  (`/Engine/EditorBlueprintResources/StandardMacros.IsValid` (`PrimitiveComponent.GetMaterial` HeadComp _returnvalue)
    (:`Is Valid`
      (bind _returnvalue_2 (`PrimitiveComponent.CreateDynamicMaterialInstance` HeadComp _returnvalue "/Game/Fab_Assets/AnimeCharacters/Materials/m_EyeEmote.m_EyeEmote" "None"))
      (set `self.EyeEmoteDynaMat` _returnvalue_2))
    (:`Is Not Valid`
      _))
  (return))

(fn `GetLookingValues`
  (returns (IsLooking :type Boolean) (`Look Vector` :type "Vector Structure"))
  (bind _looking_actor (`self.Looking Actor`)
    (:`then`
      (if (`self.Is Looking`)
        (bind _point (message `/Game/Fab_Assets/AnimeCharacters/Blueprints/Misc/bp_AnimeAnimationInterface.GetAnimLookPoint` _looking_actor))
        (`/Engine/EditorBlueprintResources/StandardMacros.IsValid` _point
          (:`Is Valid`
            (return true (`SceneComponent.K2_GetComponentLocation` _point)))
          (:`Is Not Valid`
            (return true (`Actor.K2_GetActorLocation` _looking_actor))))
        (else
          _)))
    (:`else`
      _))
  (return false (0.0 0.0 0.0)))

(fn `QuickSetAnimationValues`
  (params (`Is Looking` :type Boolean) (`Looking Actor` :type "Actor Object Reference") (`Eye Look` :type "Vector2D Structure") (CurrentExpression :type "/Game/Fab_Assets/AnimeCharacters/Blueprints/e_FacialExpressions Enum" :default "NewEnumerator0") (`Eye Emote` :type "/Game/Fab_Assets/AnimeCharacters/Blueprints/e_EyeEmote Enum" :default "NewEnumerator0") (`Is Talking` :type Boolean))
  (set `self.Is Looking` `Is Looking`)
  (set `self.Looking Actor` `Looking Actor`)
  (set `self.Eye Look` `Eye Look`)
  (set `self.Expression` CurrentExpression)
  (set `self.Eye Emote` `Eye Emote`)
  (set `self.Is Talking` `Is Talking`))

(fn `SetHeadComponent`
  (params (HeadComp :type "SkeletalMeshComponent Object Reference"))
  (set `self.HeadComp` HeadComp))

(fn `Update Emote Texture`
  (bind _eye_emote (`self.Eye Emote`))
  (bind _eyeemotedynamat (`self.EyeEmoteDynaMat`))
  (bind (_value _returnvalue) (`BlueprintMapLibrary.Map_Find` (`self.Eye Emote Textures`) _eye_emote))
  (bind _returnvalue_2 (and _returnvalue (`|EnumInequality` _eye_emote "NewEnumerator0")))
  (bind _headcomp (`self.HeadComp`)
    (:`then`
      (`/Engine/EditorBlueprintResources/StandardMacros.IsValid` _eyeemotedynamat
        (:`Is Valid`
          _)
        (:`Is Not Valid`
          (`self.CreateEyeEmoteDynamicMaterial` _headcomp)))
      (`SkeletalMeshComponent.SetMorphTarget` (`self.HeadComp`) "Eye_Override" (`KismetMathLibrary.Conv_BoolToDouble` _returnvalue_2) true)
      (if _returnvalue_2
        (`MaterialInstanceDynamic.SetTextureParameterValue` _eyeemotedynamat "Texture" _value)))
    (:`else`)))