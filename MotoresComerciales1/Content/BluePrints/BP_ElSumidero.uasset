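; BP_ElSumidero is an unfinished projectile spawner actor.
; BeginPlay waits briefly, then calls SpawnTime, which is an empty function.
; A separate Spawn event runs an empty loop over the projectile count and prints a debug message.
; A disconnected SpawnActor node, with no class shown, would use random reachable points around the actor and index-based yaw offsets, but never executes.
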(event `self.ReceiveBeginPlay`
  (`KismetSystemLibrary.Delay` 2.0)
  (`self.spawnTime`))

(event `Spawn`
  (for _index (range (+ (- (`self.ProyectileAmount`) 0) 1))
    _)
  (`KismetSystemLibrary.PrintText` "Hello"))

(fn `spawnTime`)

(fn `UserConstructionScript`)