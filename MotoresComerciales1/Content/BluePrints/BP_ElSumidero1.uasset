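; BP_ElSumidero1 is a spawner actor meant to create BP_DummyNPC instances periodically within a time window.
; BeginPlay creates a looping Spawn timer but immediately clears it, so as wired no spawning occurs.
; Spawn picks a random reachable point near the actor while game time is within InitTime and EndTime, otherwise clearing the timer.
; The nodes computing that window from Duración are disconnected.
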(event `self.ReceiveBeginPlay`
  (bind _returnvalue (`KismetSystemLibrary.K2_SetTimerDelegate` (delegate `Spawn`) 2.0 true))
  (bind _output_get (set `self.Time Handler` _returnvalue))
  (`KismetSystemLibrary.K2_ClearAndInvalidateTimerHandle` _output_get :!label _label))

(event `Spawn`
  (bind _returnvalue (`KismetSystemLibrary.GetGameTimeInSeconds`))
  (if (and (>= _returnvalue (`self.InitTime`)) (<= _returnvalue (`self.EndTime`)))
    (`|SpawnActorFromClass` "/Game/ThirdPerson/Blueprints/BP_DummyNPC.BP_DummyNPC_C" (`KismetMathLibrary.MakeTransform` (`NavigationSystemV1.K2_GetRandomReachablePointInRadius` (`self.K2_GetActorLocation`) 100.0 null null)) "Undefined" "MultiplyWithRoot" null null)
    (else
      (goto _label))))

(fn `UserConstructionScript`)