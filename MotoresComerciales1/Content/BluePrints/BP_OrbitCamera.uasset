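; An orbit camera pawn that the player rotates and zooms around its pivot on a spring arm.
; BeginPlay aligns control rotation to the camera, shows the cursor in Game and UI mode, and sets ViewPitchMax twice, leaving ViewPitchMin untouched.
; Enhanced Input drives controller yaw and inverted pitch, which the spring arm follows.
; Tick lerp-smooths the zoom input into arm length changes, clamped between minimum and maximum distances.
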(event `self.ReceiveBeginPlay`
  (bind _returnvalue (`GameplayStatics.GetPlayerController` 0))
  (bind _playercameramanager (`PlayerController.PlayerCameraManager` (`GameplayStatics.GetPlayerController` 0)))
  (`Controller.SetControlRotation` (`self.GetController`) (`SceneComponent.K2_GetComponentRotation` (`self.Camera`)))
  (set `SpringArmComponent.bUsePawnControlRotation` true (`self.SpringArm`))
  (set `PlayerCameraManager.ViewPitchMax` 80.0 _playercameramanager)
  (set `PlayerCameraManager.ViewPitchMax` 30.0 _playercameramanager)
  (set `PlayerController.bShowMouseCursor` true _returnvalue)
  (`WidgetBlueprintLibrary.SetInputMode_GameAndUIEx` _returnvalue null))

(event `EnhancedInput|/Game/BluePrints/IA_OrbitCamera`
  (params (ActionValue :type "Vector2D Structure") (ElapsedSeconds :type "Float (double-precision)") (TriggeredSeconds :type "Float (double-precision)") (InputAction :type "InputAction Object Reference" :default "/Game/BluePrints/IA_OrbitCamera.IA_OrbitCamera"))
  (:`Triggered`
    (`self.AddControllerYawInput` ActionValue_X)
    (`self.AddControllerPitchInput` (* ActionValue_Y -1.0))))

(event `self.ReceiveTick`
  (params (DeltaSeconds :type "Float (single-precision)"))
  (bind _springarm (`self.SpringArm`))
  (bind _output_get (set `self.ZoomDelta` (`KismetMathLibrary.Lerp` (`self.ZoomDelta`) (`|GetInputActionValue`) 0.1)))
  (set `SpringArmComponent.TargetArmLength` (`KismetMathLibrary.FClamp` (+ (* _output_get 100.0) (`SpringArmComponent.TargetArmLength` _springarm)) (`self.MinCameraDistance`) (`self.MaxCameraDistance`)) _springarm))

(fn `UserConstructionScript`)