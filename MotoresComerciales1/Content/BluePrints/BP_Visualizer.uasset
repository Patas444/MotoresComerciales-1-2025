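; Item visualizer actor that previews a set of prop meshes, such as rifle, hat, boots and chest, one at a time.
; It enables player input on BeginPlay.
; E drives a looping MultiGate that hides the current mesh and shows the next.
; Q drives another looping MultiGate that swaps the rifle and lantern materials between gold, silver, emerald, diamond and their defaults through new dynamic material instances.
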(event `self.ReceiveBeginPlay`
  (`self.EnableInput` (`GameplayStatics.GetPlayerController` 0)))

(event `Key|Q`
  (params (Key :type "Key Structure"))
  (:`Pressed`
    (`|MultiGate` false true
      (:`Out 0`
        (`PrimitiveComponent.CreateDynamicMaterialInstance` (`self.Mesh_Rifle`) 0 "/Game/Resourse/M_Gold.M_Gold" "None")
        (`PrimitiveComponent.CreateDynamicMaterialInstance` (`self.Mesh_Lanter`) 0 "/Game/Resourse/M_Gold.M_Gold" "None"))
      (:`Out 1`
        (`PrimitiveComponent.CreateDynamicMaterialInstance` (`self.Mesh_Rifle`) 0 "/Game/Resourse/M_Silver.M_Silver" "None")
        (`PrimitiveComponent.CreateDynamicMaterialInstance` (`self.Mesh_Lanter`) 0 "/Game/Resourse/M_Silver.M_Silver" "None"))
      (:`Out 2`
        (`PrimitiveComponent.CreateDynamicMaterialInstance` (`self.Mesh_Rifle`) 0 "/Game/Resourse/M_Esmerald.M_Esmerald" "None")
        (`PrimitiveComponent.CreateDynamicMaterialInstance` (`self.Mesh_Lanter`) 0 "/Game/Resourse/M_Esmerald.M_Esmerald" "None"))
      (:`Out 3`
        (`PrimitiveComponent.CreateDynamicMaterialInstance` (`self.Mesh_Rifle`) 0 "/Game/Resourse/M_Diamond.M_Diamond" "None")
        (`PrimitiveComponent.CreateDynamicMaterialInstance` (`self.Mesh_Lanter`) 0 "/Game/Resourse/M_Diamond.M_Diamond" "None"))
      (:`Out 4`
        (`PrimitiveComponent.CreateDynamicMaterialInstance` (`self.Mesh_Rifle`) 0 "/Game/Fab_Assets/OldWest/VOL3/Materials/MI_Rifle_NN_01a.MI_Rifle_NN_01a" "None")
        (`PrimitiveComponent.CreateDynamicMaterialInstance` (`self.Mesh_Lanter`) 0 "/Game/Fab_Assets/OldWest/VOL3/Materials/MI_Lantern_NN_01a.MI_Lantern_NN_01a" "None")))))

(event `Key|E`
  (params (Key :type "Key Structure"))
  (:`Pressed`
    (`|MultiGate` false true 0
      (:`Out 0`
        (`SceneComponent.SetVisibility` (`self.Mesh_Rifle`) false false)
        (`SceneComponent.SetVisibility` (`self.Mesh_Hat`) true false))
      (:`Out 1`
        (`SceneComponent.SetVisibility` (`self.Mesh_Hat`) false false)
        (`SceneComponent.SetVisibility` (`self.Mesh_Boots`) true false))
      (:`Out 2`
        (`SceneComponent.SetVisibility` (`self.Mesh_Boots`) false false)
        (`SceneComponent.SetVisibility` (`self.Mesh_Holster`) true false))
      (:`Out 3`
        (`SceneComponent.SetVisibility` (`self.Mesh_Holster`) false false)
        (`SceneComponent.SetVisibility` (`self.Mesh_Satchel`) true false))
      (:`Out 4`
        (`SceneComponent.SetVisibility` (`self.Mesh_Satchel`) false false)
        (`SceneComponent.SetVisibility` (`self.Mesh_Lanter`) true false))
      (:`Out 5`
        (`SceneComponent.SetVisibility` (`self.Mesh_Lanter`) false false)
        (`SceneComponent.SetVisibility` (`self.Mesh_Food`) true false))
      (:`Out 6`
        (`SceneComponent.SetVisibility` (`self.Mesh_Food`) false false)
        (`SceneComponent.SetVisibility` (`self.Mesh_Food1`) true false))
      (:`Out 7`
        (`SceneComponent.SetVisibility` (`self.Mesh_Food1`) false false)
        (`SceneComponent.SetVisibility` (`self.Mesh_Food2`) true false))
      (:`Out 8`
        (`SceneComponent.SetVisibility` (`self.Mesh_Food2`) false false)
        (`SceneComponent.SetVisibility` (`self.Mesh_Chest`) true false))
      (:`Out 9`
        (`SceneComponent.SetVisibility` (`self.Mesh_Chest`) false false)
        (`SceneComponent.SetVisibility` (`self.Mesh_Rifle`) true false)))))

(fn `UserConstructionScript`)